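; Spawner actor that drops BP_FallingObject actors at an accelerating rate.
; BeginPlay starts a looping timer on SpawnObject, which spawns at a random X/Y within the referenced SpawnVolume's bounds and a fixed height.
; Each spawn calls AdjustSpawnTimer, which subtracts a reduction rate from the interval, clamps it and resets the timer.
; The player character is cached on BeginPlay but not used in these graphs.
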(event Custom|SpawnObject
  (bind _spawnvolume (Variables|Default|GetspawnVolume))
  (bind (_origin _boxextent) (Collision|GetActorBounds _spawnvolume false false))
  (bind _returnvalue (Math|Random|RandomPointinBoundingBox _origin _boxextent))
  (bind (_x _y) (Math|Vector|BreakVector _returnvalue))
  ;[0.15 0.15 0.15 0.5] Spawn object within the volume bounds
  (Game|SpawnActorfromClass "/Game/FallProto/BP_FallingObject.BP_FallingObject_C" (Math|Conversions|ToTransform(Vector) (Math|Vector|MakeVector _x _y 6e+02)) "Undefined" "MultiplyWithRoot" 0 0)
  (CallFunction|AdjustSpawnTimer))

(event Custom|AdjustSpawnTimer
  ;[0.15 0.15 0.15 0.5] Speeds up timer over time
  (bind _output_get (Variables|Default|SetcurrentTimeInterval (Math|Float|Clamp(Float) (- (Variables|Default|GetcurrentTimeInterval) (Variables|Default|GettimeReductionRate)) (Variables|Default|GetminTimeInterval))))
  (Utilities|Time|SetTimerbyFunctionName 0 "SpawnObject" _output_get true))

(event EventBeginPlay
  ;[0.15 0.15 0.15 0.5] Spawn Timer
  (Variables|Default|SetcurrentTimeInterval (Variables|Default|GettimeInterval))
  (Variables|Default|SetplayerCharacter (Game|GetPlayerCharacter 0))
  (Utilities|Time|SetTimerbyFunctionName 0 "SpawnObject" (Variables|Default|GetcurrentTimeInterval) true))

(event Collision|EventActorBeginOverlap
  (params (OtherActor :type Actor%20Object%20Reference)))

(fn ConstructionScript)
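; BP_FallingObject is a falling physics gem that expires after AliveTime and can be picked up by BP_ThirdPersonCharacter.
; Hard hits play a velocity-scaled ting and apply the pickup material, throttled by a delayed DoOnce reset.
; Tick infers IsOnGround from velocity change, restoring the default material while it varies.
; Character overlap destroys grounded gems; the TakeDamage branch sits behind a repeated IsOnGround check, so is effectively unreachable.
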(event OnComponentBeginOverlap(SphereCollider)
  (params (OverlappedComponent :type Primitive%20Component%20Object%20Reference) (OtherActor :type Actor%20Object%20Reference) (OtherComp :type Primitive%20Component%20Object%20Reference) (OtherBodyIndex :type Integer) (bFromSweep :type Boolean) (SweepResult :type Hit%20Result%20Structure%20%28by%20ref%29))
  (if (Variables|Default|GetisOnGround)
    (bind _asbp_third_person_character (Utilities|Casting|CastToBP_ThirdPersonCharacter OtherActor))
    (if (Variables|Default|GetisOnGround)
      (Actor|DestroyActor)
      (else
        (Default|TakeDamage _asbp_third_person_character)))))

(event EventBeginPlay
  ;[0.15 0.15 0.15 0.5] Destroy object after N seconds
  (Utilities|FlowControl|Delay (Variables|Default|GetaliveTime))
  (Actor|DestroyActor))

(event Collision|EventHit
  (params (MyComp :type Primitive%20Component%20Object%20Reference) (Other :type Actor%20Object%20Reference) (OtherComp :type Primitive%20Component%20Object%20Reference) (bSelfMoved :type Boolean) (HitLocation :type Vector :default "0, 0, 0") (HitNormal :type Vector :default "0, 0, 0") (NormalImpulse :type Vector :default "0, 0, 0") (Hit :type Hit%20Result%20Structure%20%28by%20ref%29))
  ;[0.15 0.15 0.15 0.5] Play sound when object hits the ground / determine if object is on the ground
  (if (> (Math|Vector|VectorLength NormalImpulse) 2e+02)
    (Utilities|FlowControl|DoOnce false :!label _label
      (:Completed
        (Audio|PlaySoundatLocation "/Game/FallProto/Audio/ting_01.ting_01" HitLocation "0, 0, 0" (Math|Float|Clamp(Float) (/ (Math|Vector|VectorLength (Math|Conversions|ToVector(Float) (.Z (Math|Vector|BreakVector (Transformation|GetComponentVelocity (Variables|Default|GetGem)))))) 1.2e+03) 0.0 0.7) 1.0 0.0 "/USDCore/USDDefaultAttenuation.USDDefaultAttenuation" 0 0 0)
        (Development|PrintString (Utilities|String|ToString(Boolean) (Variables|Default|GetisOnGround)) false false)
        (Variables|Default|SetisOnGround false)
        (Rendering|Material|SetMaterial (Variables|Default|GetGem) 0 "/Game/FallProto/Materials/GemPickup_MAT1.GemPickup_MAT1")
        (Utilities|FlowControl|Delay 0.31)
        (goto _label Reset)))))

(event EventTick
  (params (DeltaSeconds :type Float%20%28single-precision%29))
  ;[0.15 0.15 0.15 0.5] Determine whether the object is in the ground or not
  (bind _returnvalue (Physics|GetPhysicsLinearVelocity (Variables|Default|GetGem) "None"))
  (if (> (Math|Vector|VectorLength (- _returnvalue (Variables|Default|GetlastVelocity))) 1e+01)
    (Variables|Default|SetlastVelocity _returnvalue)
    (Rendering|Material|SetMaterial (Variables|Default|GetGem) 0 "/Game/FallProto/Materials/GemDefault_MAT.GemDefault_MAT")
    (Variables|Default|SetisOnGround false)
    (else
      (Variables|Default|SetisOnGround true))))

(fn ConstructionScript)